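; Player character Blueprint that handles death, weapon-fire feedback and an on-screen controls hint.
; On death it disables input, destroys the capsule, ragdolls the mesh and reloads L_MainLocation after three seconds.
; Inventory slot updates bind the current weapon's shoot event, which plays a rifle hip-fire montage, then a sound at the actor's location.
; Tick prints the Russian controls text every frame.
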(event Custom|OnUpdateSlots
  (bind _returnvalue (Class|PlayerCharacter|GetInventoryComponent))
  (bind _returnvalue_2 (Class|InventoryComponent|GetCurrentWeapon _returnvalue))
  (Utilities|IsValid _returnvalue_2
    (:Is%20Valid
      (EventDispatchers|AssignOnShoot _returnvalue_2 (delegate Custom|OnShoot)))))

(event Custom|OnShoot
  (Animation|Montage|PlayMontage (Variables|Character|GetMesh) "/Game/Assets/AnimStarterPack/Fire_Rifle_Hip_Montage.Fire_Rifle_Hip_Montage"
    (:then
      (Audio|PlaySoundatLocation "/Game/Assets/FPWeapon/Audio/FirstPersonTemplateWeaponFire02.FirstPersonTemplateWeaponFire02" (Transformation|GetActorLocation) "0, 0, 0" 1.0 1.0 0.0 0 0 0 0))))

(event EventOnDeathEvent
  (Input|DisableInput (Game|GetPlayerController 0))
  (Components|DestroyComponent (Variables|Default|GetCapsuleComponent))
  (Collision|SetCollisionEnabled (Variables|Character|GetMesh) "QueryAndPhysics")
  (Physics|SetSimulatePhysics (Variables|Character|GetMesh) true)
  (Utilities|FlowControl|Delay 3.0)
  (Game|OpenLevel(byName) "L_MainLocation"))

(event EventBeginPlay
  (|CallParentFunction)
  (EventDispatchers|AssignOnUpdateSlots (Class|PlayerCharacter|GetInventoryComponent) (delegate Custom|OnUpdateSlots)))

(event EventTick
  (params (DeltaSeconds :type Float%20%28single-precision%29))
  (Development|PrintString (Utilities|String|MakeLiteralString "Управление: 
Ходить - ПКМ на нужную точку. 
Стрелять - ЛКМ на нужную точку. 
Перезарядка - R. 
Пауза - ESC или P. 
 
Чтобы подобрать предмет подойдите к нему, 
наведитесь и нажмите Е. 
 
Чтобы использовать предмет или поменять  
оружие - нажмите на необходимую цифру слота. 
 
Чтобы выбросить предмет - нажмите Shift 
и необходимую цифру слота.") true true "(R=1.000000,G=0.000000,B=1.000000,A=1.000000)" DeltaSeconds))

(fn ConstructionScript)