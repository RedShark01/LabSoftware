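; BP_PlayerController is the player controller that owns the player's screen UI and pause menu.
; On BeginPlay it shows W_PlayerScreen, pre-creates W_PauseMenu and binds OnLoad to the BP_GameInstance load delegate.
; The Pause input toggles game pause and adds or removes the menu from the viewport, while OnLoad unpauses and closes the menu if the game is paused.
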(event Custom|OnLoad
  ;[1 1 1] Set widgets and add delegate On Load
  (if (Game|IsGamePaused)
    (Game|SetGamePaused false)
    (Widget|RemovefromParent (Variables|Default|GetPauseMenu))))

(event EventBeginPlay
  ;[1 1 1] Set widgets and add delegate On Load
  (bind _returnvalue (UserInterface|CreateWidget "/Game/Widgets/W_PlayerScreen.W_PlayerScreen_C" self))
  (UserInterface|Viewport|AddtoViewport _returnvalue 0)
  (bind _returnvalue_2 (UserInterface|CreateWidget "/Game/Widgets/W_PauseMenu.W_PauseMenu_C" self))
  (Variables|Default|SetPauseMenu _returnvalue_2)
  (bind _asbp_game_instance (Utilities|Casting|CastToBP_GameInstance (Game|GetGameInstance)))
  (EventDispatchers|AssignOnLoad _asbp_game_instance (delegate Custom|OnLoad)))

(event Input|ActionEvents|InputActionPause
  (params (Key :type Key%20Structure))
  (bind _pausemenu (Variables|Default|GetPauseMenu))
  ;[1 1 1] Pause game
  (:Pressed
    (bind _returnvalue (Game|SetGamePaused (not (Game|IsGamePaused))))
    (if _returnvalue
      (UserInterface|Viewport|AddtoViewport _pausemenu 0)
      (else
        (Widget|RemovefromParent _pausemenu)))))

(fn ConstructionScript)